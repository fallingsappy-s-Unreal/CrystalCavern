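; Player pawn that rolls a physics static mesh, likely a ball, and restarts the level when it takes any damage.
; Movement axes apply mass-independent torque to the mesh, scaled by ForceMultiplier.
; AdjustSpringArm sets the camera arm's length and world yaw, with pitch and roll zeroed.
; RestartLevel runs once, fades the camera out over FadeDuration, then reopens the current level.
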(event EventBeginPlay)

(event Collision|EventActorBeginOverlap
  (params (OtherActor :type Actor%20Object%20Reference)))

(event EventTick
  (params (DeltaSeconds :type Float%20%28single-precision%29)))

(event Game|Damage|EventAnyDamage
  (params (Damage :type Float%20%28single-precision%29) (DamageType :type Damage%20Type%20Object%20Reference) (InstigatedBy :type Controller%20Object%20Reference) (DamageCauser :type Actor%20Object%20Reference))
  (Utilities|RestartLevel))

(event Input|AxisEvents|InputAxisMoveForwards/Backwards
  (params (AxisValue :type Float%20%28single-precision%29))
  (Class|PrimitiveComponent|AddTorqueinRadians (Variables|Default|GetStaticMesh) (Math|Vector|MakeVector 0.0 (* AxisValue (Variables|Default|GetForceMultiplier)) 0.0) "None" true))

(event Input|AxisEvents|InputAxisMoveRight/Left
  (params (AxisValue :type Float%20%28single-precision%29))
  (Class|PrimitiveComponent|AddTorqueinRadians (Variables|Default|GetStaticMesh) (Math|Vector|MakeVector (* AxisValue (Variables|Default|GetForceMultiplier)) 0.0 0.0) "None" true))

(fn ConstructionScript)

(fn AdjustSpringArm
  (params (Distance :type Float%20%28single-precision%29) (Yaw :type Float%20%28single-precision%29))
  (Variables|/Script/Engine.SpringArmComponent|SetTargetArmLength (Variables|Default|GetSpringArm) Distance)
  (Transformation|SetWorldRotation (Variables|Default|GetSpringArm) (Math|Rotator|MakeRotator 0.0 0.0 Yaw) false false))