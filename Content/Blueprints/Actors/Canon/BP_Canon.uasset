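; BP_Canon is a cannon actor that automatically and repeatedly fires BP_Projectile from the moment play begins.
; After a FireRate delay, it spawns a projectile at ProjectileSpawnPoint's world location and rotation, scaled by ProjectileScale.
; The CannonFireTrack timeline then animates CannonGun along its relative Y axis, and its Cannon Fired event loops back to the delay, so firing needs no Tick.
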(event EventBeginPlay
  (Utilities|FlowControl|Delay (Variables|CanonProperties|GetFire%20Rate) :!label _label)
  (CallFunction|SpawnProjectile)
  (bind _cannon_gun_location (Timeline|Cannon%20Fire%20Track PlayFromStart)
    (:Update
      (CallFunction|MoveCannonGun _cannon_gun_location))
    (:Cannon%20Fired
      (goto _label))))

(event Collision|EventActorBeginOverlap
  (params (OtherActor :type Actor%20Object%20Reference)))

(event EventTick
  (params (DeltaSeconds :type Float%20%28single-precision%29)))

(fn ConstructionScript)

(fn SpawnProjectile
  (bind _projectile_spawn_point (Variables|Default|GetProjectile%20Spawn%20Point))
  (Game|SpawnActorfromClass "/Game/Blueprints/Actors/Projectiles/BP_Projectile.BP_Projectile_C" (Math|Transform|MakeTransform (Transformation|GetWorldLocation _projectile_spawn_point) (Transformation|GetWorldRotation _projectile_spawn_point) (Math|Conversions|ToVector(Float) (Variables|CanonProperties|GetProjectile%20Scale))) "Undefined" 0 0))

(fn MoveCannonGun
  (params (Cannon%20Gun%20Y%20Location :type Float%20%28single-precision%29))
  (Transformation|SetRelativeLocation (Variables|Default|GetCannon_Gun) (Math|Vector|MakeVector 0.0 Cannon%20Gun%20Y%20Location 0.0) false false))